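; CellWallsRise_BP is an actor that moves four cell wall components in a staggered sequence when its CellsUp event fires.
; A Sequence node starts one timeline per wall, with the first immediate and each later one held back by a progressively longer delay.
; Each timeline's vector track drives its wall's relative location without sweeping.
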(event `CellsUp`
  (`|ExecutionSequence`
    (:`then_0`
      (bind (_direction _newtrack_2) (`Timeline|Timeline`)
        (:`Update`
          (`SceneComponent.K2_SetRelativeLocation` (`self.Wall`) _newtrack_2 false false))))
    (:`then_1`
      (`KismetSystemLibrary.Delay` 2.0)
      (bind (_direction_2 _newtrack_2_2) (`Timeline|Timeline_0`)
        (:`Update`
          (`SceneComponent.K2_SetRelativeLocation` (`self.Wall2`) _newtrack_2_2 false false))))
    (:`then_2`
      (`KismetSystemLibrary.Delay` 4.0)
      (bind (_direction_3 _newtrack_2_3) (`Timeline|Timeline_1`)
        (:`Update`
          (`SceneComponent.K2_SetRelativeLocation` (`self.Wall3`) _newtrack_2_3 false false))))
    (:`then_3`
      (`KismetSystemLibrary.Delay` 6.0)
      (bind (_direction_4 _newtrack_2_4) (`Timeline|Timeline_2`)
        (:`Update`
          (`SceneComponent.K2_SetRelativeLocation` (`self.Wall4`) _newtrack_2_4 false false))))))

(fn `UserConstructionScript`)