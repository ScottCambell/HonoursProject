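; TorchFire_BP is a corridor Blueprint that switches a set of fire effects and point lights in a staggered sequence when the player enters its Box trigger.
; The overlap event filters for the player pawn, then steps through groups of Fire components and their PointLights with short Delays between them.
; Each step toggles the current state rather than setting it, with no one-shot guard, so a later entry can reverse the effect.
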(event `self.Box.OnComponentBeginOverlap`
  (params (OverlappedComponent :type "PrimitiveComponent Object Reference") (OtherActor :type "Actor Object Reference") (OtherComp :type "PrimitiveComponent Object Reference") (OtherBodyIndex :type Integer) (bFromSweep :type Boolean) (SweepResult :type "HitResult Structure (by ref)"))
  (if (== OtherActor (`GameplayStatics.GetPlayerPawn` 0))
    (`ActorComponent.ToggleActive` (`self.Fire`))
    (`ActorComponent.ToggleActive` (`self.Fire2`))
    (`SceneComponent.ToggleVisibility` (`self.PointLight`) false)
    (`SceneComponent.ToggleVisibility` (`self.PointLight3`) false)
    (`KismetSystemLibrary.Delay` 0.5)
    (`ActorComponent.ToggleActive` (`self.Fire1`))
    (`SceneComponent.ToggleVisibility` (`self.PointLight1`) false)
    (`KismetSystemLibrary.Delay` 0.5)
    (`ActorComponent.ToggleActive` (`self.Fire3`))
    (`ActorComponent.ToggleActive` (`self.Fire4`))
    (`SceneComponent.ToggleVisibility` (`self.PointLight2`) false)
    (`SceneComponent.ToggleVisibility` (`self.PointLight4`) false)
    (`KismetSystemLibrary.Delay` 0.5)
    (`ActorComponent.ToggleActive` (`self.Fire5`))
    (`SceneComponent.ToggleVisibility` (`self.PointLight5`) false)
    (`KismetSystemLibrary.Delay` 0.4)
    (`ActorComponent.ToggleActive` (`self.Fire6`))
    (`SceneComponent.ToggleVisibility` (`self.PointLight6`) false)
    (`KismetSystemLibrary.Delay` 0.4)))

(fn `UserConstructionScript`)