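; Corridor trigger actor that switches the player into and back out of a VHS-style camera mode, using two one-shot overlap boxes.
; The first box turns on the flashlight and 4:3 resolution, then after a delayed fade toggles post-process, adds the VHS overlay and opens a Tick-fed gate driving character headbob.
; The second box reverses these changes behind another camera fade, restoring 16:9 and closing the headbob gate.
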(event `self.Box.OnComponentBeginOverlap`
  (params (OverlappedComponent :type "PrimitiveComponent Object Reference") (OtherActor :type "Actor Object Reference") (OtherComp :type "PrimitiveComponent Object Reference") (OtherBodyIndex :type Integer) (bFromSweep :type Boolean) (SweepResult :type "HitResult Structure (by ref)"))
  ; camera effects transition
  (`/Engine/EditorBlueprintResources/StandardMacros.DoOnce` false
    (:`Completed`
      (`|ExecutionSequence`
        (:`then_0`
          (bind _returnvalue (`GameplayStatics.GetActorOfClass` "/Game/FirstPerson/Blueprints/BP_FirstPersonCharacter.BP_FirstPersonCharacter_C"))
          (`/Game/FirstPerson/Blueprints/BP_FirstPersonCharacter.TurnOnFlashlight` _returnvalue)
          (`/Game/FirstPerson/Blueprints/BP_FirstPersonCharacter.Resolution4:3Change` _returnvalue)
          (`KismetSystemLibrary.Delay` 4.0)
          (`PlayerCameraManager.StartCameraFade` :`self` (`GameplayStatics.GetPlayerCameraManager` 0) :`ToAlpha` 1.0 :`Duration` 1.0 :`bShouldFadeAudio` true :`bHoldWhenFinished` true)
          (`KismetSystemLibrary.Delay` 1.0)
          (`PlayerCameraManager.StartCameraFade` :`self` (`GameplayStatics.GetPlayerCameraManager` 0) :`FromAlpha` 1.0 :`Duration` 0.5 :`bShouldFadeAudio` true :`bHoldWhenFinished` true))
        (:`then_1`
          (`KismetSystemLibrary.Delay` 5.0)
          (`SceneComponent.ToggleVisibility` (`self.PostProcess`) false))
        (:`then_2`
          (`KismetSystemLibrary.Delay` 5.0)
          (bind _returnvalue_2 (`|CreateWidget` "/Game/Films/Overlays/VHSOverlay_W.VHSOverlay_W_C"))
          (`UserWidget.AddToViewport` _returnvalue_2 0))
        (:`then_3`
          (`KismetSystemLibrary.Delay` 5.0)
          (goto _label :!via `Open`))))))

(event `self.ReceiveTick`
  (params (DeltaSeconds :type "Float (single-precision)"))
  ; camera effects transition
  (`/Engine/EditorBlueprintResources/StandardMacros.Gate` true :!label _label
    (:`Exit`
      (bind _returnvalue (`GameplayStatics.GetActorOfClass` "/Game/FirstPerson/Blueprints/BP_FirstPersonCharacter.BP_FirstPersonCharacter_C"))
      (`/Game/FirstPerson/Blueprints/BP_FirstPersonCharacter.Headbob` _returnvalue))))

(event `StopHeadbob`
  ; camera effects transition
  (goto _label :!via `Close`))

(event `self.Box1.OnComponentBeginOverlap`
  (params (OverlappedComponent :type "PrimitiveComponent Object Reference") (OtherActor :type "Actor Object Reference") (OtherComp :type "PrimitiveComponent Object Reference") (OtherBodyIndex :type Integer) (bFromSweep :type Boolean) (SweepResult :type "HitResult Structure (by ref)"))
  ; turn off camera effects
  (`/Engine/EditorBlueprintResources/StandardMacros.DoOnce` false
    (:`Completed`
      (`|ExecutionSequence`
        (:`then_0`
          (`KismetSystemLibrary.Delay` 1.0)
          (bind _returnvalue (`GameplayStatics.GetActorOfClass` "/Game/FirstPerson/Blueprints/BP_FirstPersonCharacter.BP_FirstPersonCharacter_C"))
          (`/Game/FirstPerson/Blueprints/BP_FirstPersonCharacter.Turn off Flashlight` _returnvalue)
          (`/Game/FirstPerson/Blueprints/BP_FirstPersonCharacter.Resolution16:9Change` _returnvalue)
          (`Widget.RemoveFromParent` (stale `self.Box.OnComponentBeginOverlap` _returnvalue_2))
          (`self.StopHeadbob`))
        (:`then_1`
          (`KismetSystemLibrary.Delay` 1.0)
          (`SceneComponent.ToggleVisibility` (`self.PostProcess`) false))
        (:`then_2`
          (`PlayerCameraManager.StartCameraFade` :`self` (`GameplayStatics.GetPlayerCameraManager` 0) :`ToAlpha` 1.0 :`Duration` 1.0 :`bShouldFadeAudio` true :`bHoldWhenFinished` true)
          (`KismetSystemLibrary.Delay` 1.0)
          (`PlayerCameraManager.StartCameraFade` :`self` (`GameplayStatics.GetPlayerCameraManager` 0) :`FromAlpha` 1.0 :`Duration` 0.5 :`bShouldFadeAudio` true :`bHoldWhenFinished` true))))))

(fn `UserConstructionScript`)