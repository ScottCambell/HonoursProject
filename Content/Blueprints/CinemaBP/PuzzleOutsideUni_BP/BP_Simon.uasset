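; Simon-says musical puzzle actor that plays random note sequences on linked BP_Stand actors and checks the player's repeats across configurable levels.
; A box overlap moves a barrier and starts a level, building and playing the sequence through self-calling events with delays.
; Mistakes trigger errors and a new sequence; clearing the last level removes keys and the invisible wall with effects.
; The construction script caps note counts to stand count where duplicates are disallowed.
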(event `StartLevel`
  ;[1 1 1] Start new level
  (`KismetArrayLibrary.Array_Clear` (`self.PlayerSequence`))
  (set `self.CurrentNote` 0)
  (set `self.IsPlayersTurn` false)
  (`self.CreateSimonSequence`))

(event `self.StartNiagara.OnComponentBeginOverlap`
  (params (OverlappedComponent :type "PrimitiveComponent Object Reference") (OtherActor :type "Actor Object Reference") (OtherComp :type "PrimitiveComponent Object Reference") (OtherBodyIndex :type Integer) (bFromSweep :type Boolean) (SweepResult :type "HitResult Structure (by ref)"))
  ;[1 1 1 0.5] Music Notes Niagara Start
  (`ActorComponent.Activate` (`self.FogDust_NS`) false))

(event `self.ReceiveBeginPlay`
  ;[1 1 1] On begin play set reference in stands
  (for _array_element (`self.Stands`)
    (`/Engine/EditorBlueprintResources/StandardMacros.IsValid` _array_element
      (:`Is Valid`
        (set `/Game/Blueprints/CinemaBP/PuzzleOutsideUni_BP/BP_Stand.SimonMain_Ref` self _array_element)))))

(event `PlaySimonSequence`
  ;[1 1 1 0.5] Simon is Playing
  (`/Game/Blueprints/CinemaBP/PuzzleOutsideUni_BP/BP_Stand.PlayNote` (`|GetArrayItem` (`self.Stands`) (`|GetArrayItem` (`self.SimonSequence`) (`self.CurrentNote`))))
  (`KismetSystemLibrary.Delay` (`.TimeBetweenNotes_6_E5C7F82D42676A19E95BA8A4F3057531` (break `/Game/Blueprints/CinemaBP/PuzzleOutsideUni_BP/SimonLevelStructure` (`|GetArrayItem` (`self.LevelSettings`) (`self.CurrentLevel`)))))
  (`/Engine/EditorBlueprintResources/StandardMacros.IncrementInt` (`self.CurrentNote`)
    (:`  `
      (if (< (`self.CurrentNote`) (`KismetArrayLibrary.Array_Length` (`self.SimonSequence`)))
        (`self.PlaySimonSequence`)
        (else
          (set `self.IsPlayersTurn` true))))))

(event `self.Box.OnComponentBeginOverlap`
  (params (OverlappedComponent :type "PrimitiveComponent Object Reference") (OtherActor :type "Actor Object Reference") (OtherComp :type "PrimitiveComponent Object Reference") (OtherBodyIndex :type Integer) (bFromSweep :type Boolean) (SweepResult :type "HitResult Structure (by ref)"))
  ;[1 1 1] Overlap event start level
  (if (and (`KismetSystemLibrary.DoesImplementInterface` OtherActor "/Game/Blueprints/CinemaBP/PuzzleOutsideUni_BP/BP_Player1.BP_Player1_C") (not (`self.isPlaying`)))
    (set `self.isPlaying` true)
    (`KismetSystemLibrary.Delay` 1.0)
    (bind (_direction _newtrack_0) (`Timeline|Timeline`)
      (:`Update`
        (`SceneComponent.K2_SetRelativeLocation` (`self.Invisible Barrier`) _newtrack_0 false false)
        (`self.StartLevel`)))))

(event `PlayerPlayedNote`
  (params (Note :type Integer))
  ;[1 1 1] The Player begins inputting a response. If wrong, starts again. If right Door opens
  (set `self.isPlaying` false)
  (bind _returnvalue (`KismetArrayLibrary.Array_Add` (`self.PlayerSequence`) Note))
  (if (== Note (`|GetArrayItem` (`self.SimonSequence`) _returnvalue))
    (`/Game/Blueprints/CinemaBP/PuzzleOutsideUni_BP/BP_Stand.PlayNote` (`|GetArrayItem` (`self.Stands`) Note))
    (if (>= (`KismetArrayLibrary.Array_Length` (`self.PlayerSequence`)) (`KismetArrayLibrary.Array_Length` (`self.SimonSequence`)))
      (if (< (`self.CurrentLevel`) (`KismetArrayLibrary.Array_LastIndex` (`self.LevelSettings`)))
        (`/Engine/EditorBlueprintResources/StandardMacros.IncrementInt` (`self.CurrentLevel`)
          (:`  `
            (`WidgetLayoutLibrary.RemoveAllWidgets`)
            (`KismetSystemLibrary.Delay` 0.0)
            (`self.StartLevel`)))
        (else
          ;;[1 1 1] Level Complete
          (`KismetSystemLibrary.PrintString` "Player wins")
          (`WidgetLayoutLibrary.RemoveAllWidgets`)
          ; Animations of keyboard going away
          (`ActorComponent.Activate` (`self.ShockwavePuzzleWin_NS`) false)
          (`|ExecutionSequence`
            (:`then_0`
              (bind (_direction _newtrack_0) (`Timeline|move over keys`)
                (:`Update`
                  (`SceneComponent.K2_SetRelativeLocation` (`self.Invisible wall`) _newtrack_0 false true)
                  (`ActorComponent.Deactivate` (`self.FogDust_NS`))
                  (`KismetSystemLibrary.Delay` 4.0)
                  (`ActorComponent.K2_DestroyComponent` (`self.Invisible wall`)))))
            (:`then_1`
              (bind _outactors (`GameplayStatics.GetAllActorsOfClass` "/Game/Blueprints/CinemaBP/PuzzleOutsideUni_BP/BP_Stand.BP_Stand_C"))
              (`/Game/Blueprints/CinemaBP/PuzzleOutsideUni_BP/BP_Stand.MoveKey` _outactors)
              (`KismetSystemLibrary.Delay` 3.0)
              (bind _outactors_2 (`GameplayStatics.GetAllActorsOfClass` "/Game/Blueprints/CinemaBP/PuzzleOutsideUni_BP/BP_BlackKey.BP_BlackKey_C"))
              (`/Game/Blueprints/CinemaBP/PuzzleOutsideUni_BP/BP_BlackKey.BlackKeysBurn` _outactors_2))
            (:`then_2`
              (bind (_direction_2 _newtrack_0_2) (`Timeline|Timeline_1`)
                (:`Update`
                  (`SceneComponent.K2_SetRelativeLocation` (`self.Box`) _newtrack_0_2 false false))))
            (:`then_3`
              (`KismetSystemLibrary.Delay` 0.5)
              (`GameplayStatics.PlaySoundAtLocation` "/Game/Audio/Puzzle1/Puzzle_complete.Puzzle_complete" (0.0 0.0 0.0) (struct) 1.0 1.0 0.0 null null null null)))))
      (else
        (set `self.IsPlayersTurn` true)))
    (else
      (for _array_element (`self.Stands`)
        (`/Game/Blueprints/CinemaBP/PuzzleOutsideUni_BP/BP_Stand.PlayError` _array_element)
        (`WidgetLayoutLibrary.RemoveAllWidgets`))
      (`KismetSystemLibrary.Delay` 2.0)
      (`self.StartLevel`))))

(event `AddNote`
  (bind ((`NumberOfNotes_2_09023BF24A3E01D7F1FD06BDD824AA8C` _numberofnotes) (`CanDuplicateNotes_9_A034164C4D823A0F80894BB71D42797D` _canduplicatenotes)) (break `/Game/Blueprints/CinemaBP/PuzzleOutsideUni_BP/SimonLevelStructure` (`|GetArrayItem` (`self.LevelSettings`) (`self.CurrentLevel`))))
  ;[1 1 1] Create Random Sequence based on level settings
  (if (> (`KismetArrayLibrary.Array_Length` (`self.Stands`)) 0) :!label _label
    (if _canduplicatenotes
      (`KismetArrayLibrary.Array_Add` (`self.SimonSequence`) (`KismetMathLibrary.RandomIntegerInRange` 0 (`KismetArrayLibrary.Array_LastIndex` (`self.Stands`))))
      (else
        (`KismetArrayLibrary.Array_AddUnique` (`self.SimonSequence`) (`KismetMathLibrary.RandomIntegerInRange` 0 (`KismetArrayLibrary.Array_LastIndex` (`self.Stands`))))))
    (if (< (`KismetArrayLibrary.Array_Length` (`self.SimonSequence`)) _numberofnotes)
      (`KismetSystemLibrary.Delay` 0.0)
      (`self.AddNote`)
      (else
        (`KismetSystemLibrary.Delay` 1.0)
        (`self.PlaySimonSequence`)))))

(event `CreateSimonSequence`
  ;[1 1 1] Create Random Sequence based on level settings
  (`KismetArrayLibrary.Array_Clear` (`self.SimonSequence`))
  (goto _label))

(fn `UserConstructionScript`
  (bind _returnvalue (`KismetArrayLibrary.Array_Length` (`self.Stands`)))
  (for (_array_element _array_index) (`self.LevelSettings`)
    (bind ((`NumberOfNotes_2_09023BF24A3E01D7F1FD06BDD824AA8C` _numberofnotes) (`CanDuplicateNotes_9_A034164C4D823A0F80894BB71D42797D` _canduplicatenotes)) (break `/Game/Blueprints/CinemaBP/PuzzleOutsideUni_BP/SimonLevelStructure` _array_element))
    (if _canduplicatenotes
      _
      (elif (> _numberofnotes _returnvalue)
        (bind _structout (setmembers `/Game/Blueprints/CinemaBP/PuzzleOutsideUni_BP/SimonLevelStructure` :`StructRef` _array_element :`NumberOfNotes` _returnvalue))
        (`KismetArrayLibrary.Array_Set` (`self.LevelSettings`) _array_index _structout)))))