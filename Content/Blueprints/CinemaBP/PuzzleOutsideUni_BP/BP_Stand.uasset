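; BP_Stand is one pad in a Simon-style note puzzle, with its own sound and colour.
; During the player's turn, interaction reports its Index to SimonMainRef, and look-at briefly shows a cursor widget and overlay, cleared by a retriggerable delay.
; PlayNote plays the sound and pulses the dynamic material's glow, while PlayError temporarily swaps in a mistake sound and red glow.
; MoveKey moves the cube along a timeline.
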(event `MoveKey`
  (bind (_direction _newtrack_0) (`Timeline|Timeline`)
    (:`Update`
      (`SceneComponent.K2_SetRelativeLocation` (`self.Cube`) _newtrack_0 false false))))

(event `self.ReceiveBeginPlay`
  (`AudioComponent.SetSound` (`self.Audio`) (`self.Sound`)))

(event `/Game/Blueprints/CinemaBP/PuzzleOutsideUni_BP/BP_Interact1.OnInteract`
  (params (Actor :type "Actor Object Reference"))
  (if (`KismetSystemLibrary.DoesImplementInterface` Actor "/Game/Blueprints/CinemaBP/PuzzleOutsideUni_BP/BP_Player1.BP_Player1_C")
    (bind _simonmain_ref (`self.SimonMain_Ref`)
      (:`then`
        ;[1 1 1] IsPlayersTurn
        (if (`/Game/Blueprints/CinemaBP/PuzzleOutsideUni_BP/BP_Simon.IsPlayersTurn` _simonmain_ref)
          (`/Game/Blueprints/CinemaBP/PuzzleOutsideUni_BP/BP_Simon.PlayerPlayedNote` (`self.SimonMain_Ref`) (`self.Index`))))
      (:`else`))))

(event `PlayNote`
  (`AudioComponent.Play` (`self.Audio`) 0.0)
  (`MaterialInstanceDynamic.SetScalarParameterValue` (`self.DynamicMaterial`) "Intensity" 5.0)
  (`KismetSystemLibrary.Delay` 1.0)
  (`MaterialInstanceDynamic.SetScalarParameterValue` (`self.DynamicMaterial`) "Intensity" 0.0))

(event `/Game/Blueprints/CinemaBP/PuzzleOutsideUni_BP/BP_Interact1.OnLookAt`
  (params (Actor :type "Actor Object Reference"))
  (bind _simonmain_ref (`self.SimonMain_Ref`)
    (:`then`
      ;[1 1 1] IsPlayersTurn
      (if (`/Game/Blueprints/CinemaBP/PuzzleOutsideUni_BP/BP_Simon.IsPlayersTurn` _simonmain_ref)
        (bind _returnvalue (`|CreateWidget` "/Game/Blueprints/CinemaBP/PuzzleOutsideUni_BP/PuzzleCursor_BP.PuzzleCursor_BP_C"))
        (`UserWidget.AddToViewport` _returnvalue 0)
        (`MeshComponent.SetOverlayMaterial` (`self.Cube`) "/Game/Blueprints/CinemaBP/PuzzleOutsideUni_BP/M_Overlay.M_Overlay")
        (`KismetSystemLibrary.RetriggerableDelay` 0.11)
        (`MeshComponent.SetOverlayMaterial` (`self.Cube`) null)
        (`WidgetLayoutLibrary.RemoveAllWidgets`)))
    (:`else`)))

(event `PlayError`
  (`/Engine/EditorBlueprintResources/StandardMacros.DoOnce` false :!label _label
    (:`Completed`
      ;[1 1 1] Error Sound!
      (`AudioComponent.SetSound` (`self.Audio`) "/Game/Audio/Puzzle1/MistakeNoise_MS.MistakeNoise_MS")
      (`AudioComponent.Play` (`self.Audio`) 0.0)
      (`MaterialInstanceDynamic.SetVectorParameterValue` (`self.DynamicMaterial`) "Colour" (struct :`R` 0.554 :`G` 0.012343 :`A` 1.0))
      (`MaterialInstanceDynamic.SetScalarParameterValue` (`self.DynamicMaterial`) "Intensity" 10.0)
      ;[1 1 1] Depends on audio length
      (`KismetSystemLibrary.Delay` 3.0)
      (`AudioComponent.Stop` (`self.Audio`))
      (`MaterialInstanceDynamic.SetScalarParameterValue` (`self.DynamicMaterial`) "Intensity" 0.0)
      (`MaterialInstanceDynamic.SetVectorParameterValue` (`self.DynamicMaterial`) "Colour" (`self.Colour`))
      (`AudioComponent.SetSound` (`self.Audio`) (`self.Sound`))
      (goto _label :!via `Reset`))))

(fn `UserConstructionScript`
  (bind _returnvalue (`PrimitiveComponent.CreateDynamicMaterialInstance` (`self.Cube`) 0 "/Game/Blueprints/CinemaBP/PuzzleOutsideUni_BP/M_Colour.M_Colour" "None"))
  (bind _output_get (set `self.DynamicMaterial` _returnvalue))
  (`MaterialInstanceDynamic.SetVectorParameterValue` _output_get "Colour" (`self.Colour`)))