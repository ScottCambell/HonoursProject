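; BP_BlackKey is a puzzle key prop that dissolves away when its BlackKeysBurn event is called.
; The event activates the DisappearingBlackKeysNS effect and plays a timeline that drives the Progress material parameter on the Cube component.
; A delay on the timeline's update then destroys the Cube.
; The stored DissolveKeys_MI dynamic instance is never applied, as Progress is set directly on the Cube's materials.
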(event `BlackKeysBurn`
  (bind _returnvalue (`KismetMaterialLibrary.CreateDynamicMaterialInstance` "/Game/Materials/PuzzleMaterials/DissolveKeys_MI.DissolveKeys_MI" "Progress"))
  (set `self.MI_Dissolve` _returnvalue)
  (`MeshComponent.SetScalarParameterValueOnMaterials` (`self.Cube`) "Progress" 0.2)
  (`ActorComponent.Activate` (`self.Disappearing_BlackKeys_NS`) false)
  (bind (_direction _newtrack_0) (`Timeline|Timeline`)
    (:`Update`
      (`MeshComponent.SetScalarParameterValueOnMaterials` (`self.Cube`) "Progress" _newtrack_0)
      (`KismetSystemLibrary.Delay` 4.0)
      (`ActorComponent.K2_DestroyComponent` (`self.Cube`)))))

(fn `UserConstructionScript`)