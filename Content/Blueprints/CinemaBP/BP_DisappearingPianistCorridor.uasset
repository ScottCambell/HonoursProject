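; Cinematic Blueprint for a corridor pianist that dissolves away when something overlaps its trigger box.
; After a short delay, meant to become an audio-length wait, a timeline drives the "Progress!" scalar on the static mesh's materials.
; A second delayed branch activates the DisappearingPianistNS effect during the dissolve.
; The dynamic dissolve material it creates is stored but never applied, and the overlap has no once-only guard.
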(event `self.Box Collision.OnComponentBeginOverlap`
  (params (OverlappedComponent :type "PrimitiveComponent Object Reference") (OtherActor :type "Actor Object Reference") (OtherComp :type "PrimitiveComponent Object Reference") (OtherBodyIndex :type Integer) (bFromSweep :type Boolean) (SweepResult :type "HitResult Structure (by ref)"))
  ; Put audio first then use delay for audio length
  (`KismetSystemLibrary.Delay` 1.0)
  (bind _returnvalue (`KismetMaterialLibrary.CreateDynamicMaterialInstance` "/Game/CinemaObjects/stichless-mannequin/source/MI_PianoPlayerdissolve.MI_PianoPlayerdissolve" "Progress!"))
  (set `self.Dissolve` _returnvalue)
  (`MeshComponent.SetScalarParameterValueOnMaterials` (`self.StaticMesh`) "Progress!" 0.0)
  (`|ExecutionSequence`
    (:`then_0`
      (bind (_direction _newtrack_0) (`Timeline|Timeline`)
        (:`Update`
          (`MeshComponent.SetScalarParameterValueOnMaterials` (`self.StaticMesh`) "Progress!" _newtrack_0))))
    (:`then_1`
      (`KismetSystemLibrary.Delay` 1.0)
      (`ActorComponent.Activate` (`self.DisappearingPianist_NS`) false))))

(fn `UserConstructionScript`)