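; Portal actor in a corridor that moves the first-person player to the conveyor belt level.
; Overlapping the outer trigger box reveals the portal mesh and activates its effect, then enables the inner box's collision after a timed delay.
; A separate event switches that inner collision off so it is not triggered early.
; Once enabled, the inner box loads the level shortly after the player character overlaps it.
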(event `disable collision`
  ; Stop collision box being triggered early
  (`PrimitiveComponent.SetCollisionEnabled` (`self.Box`) "NoCollision"))

(event `self.Box1.OnComponentBeginOverlap`
  (params (OverlappedComponent :type "PrimitiveComponent Object Reference") (OtherActor :type "Actor Object Reference") (OtherComp :type "PrimitiveComponent Object Reference") (OtherBodyIndex :type Integer) (bFromSweep :type Boolean) (SweepResult :type "HitResult Structure (by ref)"))
  (`SceneComponent.SetVisibility` (`self.Portal`) true false)
  (`ActorComponent.Activate` (`self.PortalEffect`) false)
  (`KismetSystemLibrary.Delay` 15.0)
  ; Turn back on box collision after sequence
  (`PrimitiveComponent.SetCollisionEnabled` (`self.Box`) "QueryAndPhysics"))

(event `self.Box.OnComponentBeginOverlap`
  (params (OverlappedComponent :type "PrimitiveComponent Object Reference") (OtherActor :type "Actor Object Reference") (OtherComp :type "PrimitiveComponent Object Reference") (OtherBodyIndex :type Integer) (bFromSweep :type Boolean) (SweepResult :type "HitResult Structure (by ref)"))
  (cast `/Game/FirstPerson/Blueprints/BP_FirstPersonCharacter` OtherActor)
  ; put sound here
  (`KismetSystemLibrary.Delay` 0.2)
  (`GameplayStatics.OpenLevel` "ConveyorBeltLevel"))

(fn `UserConstructionScript`)